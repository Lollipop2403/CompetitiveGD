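; Pawn chess piece Blueprint that highlights the squares a pawn can move to or capture on.
; ShowPossibleMoves sets the forward direction from the active player's color, resets the en passant flag and clears old highlights.
; It queries GameMode occupancy to mark one step forward, a double step on the initial move if unblocked, and enemy-occupied forward diagonals.
; It returns IsKing; en passant captures are not computed here.
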(fn `HighlightPawnSquare`
  (params (X :type Integer) (Y :type Integer))
  (`/Game/Blueprints/BP_GameMode.HighlightSquare` (`self.GameModeRef`) X Y))

(fn `SetAttackSquareLeft`
  (bind _returnvalue (- (`self.Y`) 1))
  (bind _returnvalue_2 (+ (`self.X`) (`self.DirectionValue`)))
  (bind (_chesspiece _isoccupied _isoccupiedbyfriend) (`/Game/Blueprints/BP_GameMode.GetOccupant` (`self.GameModeRef`) _returnvalue_2 _returnvalue (`self.Color`)))
  (if (and _isoccupied (not _isoccupiedbyfriend))
    (`self.HighlightPawnSquare` _returnvalue_2 _returnvalue)))

(fn `SetAttackSquareRight`
  (bind _returnvalue (+ (`self.X`) (`self.DirectionValue`)))
  (bind _returnvalue_2 (+ (`self.Y`) 1))
  (bind (_chesspiece _isoccupied _isoccupiedbyfriend) (`/Game/Blueprints/BP_GameMode.GetOccupant` (`self.GameModeRef`) _returnvalue _returnvalue_2 (`self.Color`)))
  (if (and _isoccupied (not _isoccupiedbyfriend))
    (`self.HighlightPawnSquare` _returnvalue _returnvalue_2)))

(fn `SetDirectionValue`
  (switch `/Game/Blueprints/EN_Color` (`/Game/Blueprints/BP_GameMode.GetActivePlayerColor` (`self.GameModeRef`))
    (:`NewEnumerator0`
      (set `self.DirectionValue` (`self.WhiteDirection`)))
    (:`NewEnumerator1`
      (set `self.DirectionValue` (`self.BlackDirection`)))))

(fn `SetFirstSquare`
  (returns (Success :type Boolean))
  (bind _returnvalue (+ (`self.X`) (`self.DirectionValue`)))
  (if (`.IsOccupied` (`/Game/Blueprints/BP_GameMode.GetOccupant` (`self.GameModeRef`) _returnvalue (`self.Y`) (`self.Color`)))
    (return false)
    (else
      (`self.HighlightPawnSquare` _returnvalue (`self.Y`))
      (return true))))

(fn `SetSecondSquare`
  (bind _returnvalue (+ (`self.X`) (* (`self.DirectionValue`) 2)))
  (if (and (`self.IsInitialMove`) (not (`.IsOccupied` (`/Game/Blueprints/BP_GameMode.GetOccupant` (`self.GameModeRef`) _returnvalue (`self.Y`) (`self.Color`)))))
    (`/Game/Blueprints/BP_GameMode.HighlightSquare` (`self.GameModeRef`) _returnvalue (`self.Y`))))

(fn `ShowPossibleMoves`
  (returns (IsKing :type Boolean))
  (`|ExecutionSequence`
    (:`then_0`
      (`self.SetDirectionValue`)
      (set `self.IsEnPassant` false))
    (:`then_1`
      (`/Game/Blueprints/BP_GameMode.UnHighlightSquares` (`self.GameModeRef`)))
    (:`then_2`
      (bind _success (`self.SetFirstSquare`))
      (if _success
        (`self.SetSecondSquare`)))
    (:`then_3`
      (`self.SetAttackSquareRight`))
    (:`then_4`
      (`self.SetAttackSquareLeft`))
    (:`then_5`
      (return (`self.IsKing`)))))

(fn `UserConstructionScript`
  (`parent.UserConstructionScript`))