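; Knight chess piece Blueprint that shows the squares the knight can move to on the board.
; ShowPossibleMoves has the game mode clear existing highlights, runs HighlightKnightLoop, then returns the IsKing flag.
; The loop passes the eight fixed L-shaped offsets to HighlightKnightSquare, which adds each to the piece's X and Y.
; Each resulting square goes to HighlightPotentialSquare along with the piece's Color.
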(fn `HighlightKnightLoop`
  (`|ExecutionSequence`
    (:`then_0`
      (`self.HighlightKnightSquare` 2 1)
      (`self.HighlightKnightSquare` 2 -1))
    (:`then_1`
      (`self.HighlightKnightSquare` -2 1)
      (`self.HighlightKnightSquare` -2 -1))
    (:`then_2`
      (`self.HighlightKnightSquare` 1 2)
      (`self.HighlightKnightSquare` 1 -2))
    (:`then_3`
      (`self.HighlightKnightSquare` -1 2)
      (`self.HighlightKnightSquare` -1 -2))))

(fn `HighlightKnightSquare`
  (params (XIncr :type Integer) (YIncr :type Integer))
  (locals (TempX :type Integer) (TempY :type Integer))
  (bind _output_get (set `local.TempX` (+ (`self.X`) XIncr)))
  (bind _output_get_2 (set `local.TempY` (+ YIncr (`self.Y`))))
  (`self.HighlightPotentialSquare` _output_get _output_get_2 (`self.Color`)))

(fn `ShowPossibleMoves`
  (returns (IsKing :type Boolean))
  (`|ExecutionSequence`
    (:`then_0`
      (`/Game/Blueprints/BP_GameMode.UnHighlightSquares` (`self.GameModeRef`)))
    (:`then_1`
      (`self.HighlightKnightLoop`))
    (:`then_2`
      (return (`self.IsKing`)))))

(fn `UserConstructionScript`
  (`parent.UserConstructionScript`))