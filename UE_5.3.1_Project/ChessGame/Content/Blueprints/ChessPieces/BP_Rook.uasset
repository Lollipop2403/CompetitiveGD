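; BP_Rook is a chess piece Blueprint that shows a rook's possible moves on the board.
; ShowPossibleMoves clears highlights through the game mode, highlights horizontal and vertical squares, then returns IsKing.
; It also holds king-style helpers that highlight valid squares not occupied by friends, using game mode occupancy queries, though nothing here calls them.
; An unfinished EvaluateCastlePath scans along Y for blockers, with an empty edge branch that never ends the loop.
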(fn `EvaluateCastlePath`
  (params (YIncr :type Integer))
  (locals (CanContinue :type Boolean) (IsPositive :type Boolean) (TempY :type Integer))
  (set `local.IsPositive` (> YIncr 0))
  (set `local.TempY` (`self.Y`))
  (set `local.CanContinue` true)
  (while (`local.CanContinue`)
    (set `local.TempY` (+ YIncr (`local.TempY`)))
    (if (and (< (`local.TempY`) 8) (> (`local.TempY`) 1))
      (set `local.CanContinue` (not (`.IsOccupied` (`/Game/Blueprints/BP_GameMode.GetOccupant` (`self.GameModeRef`) (`self.X`) (`local.TempY`) (`self.Color`)))))
      (elif true
        _))))

(fn `HighlightKingSquare`
  (params (XIncremented :type Integer) (YIncremented :type Integer))
  (locals (TempX :type Integer) (TempY :type Integer))
  (set `local.TempX` (+ (`self.X`) XIncremented))
  (set `local.TempY` (+ (`self.Y`) YIncremented))
  (if (`self.IsValidMoveForKing` (`local.TempX`) (`local.TempY`))
    (`self.HighlightPotentialSquare` (`local.TempX`) (`local.TempY`) (`self.Color`))))

(fn `IsValidMoveForKing`
  (params (X :type Integer) (Y :type Integer))
  (returns (IsValidMove :type Boolean))
  (bind (_chesspiece _isoccupied _isoccupiedbyfriend _isvalid) (`/Game/Blueprints/BP_GameMode.GetOccupant` (`self.GameModeRef`) X Y (`self.Color`)))
  (if _isvalid
    (if _isoccupiedbyfriend
      (return false)
      (else
        (return true)))
    (else
      (return false))))

(fn `ShowPossibleMoves`
  (returns (IsKing :type Boolean))
  (bind _color (`self.Color`))
  (`|ExecutionSequence`
    (:`then_0`
      (`/Game/Blueprints/BP_GameMode.UnHighlightSquares` (`self.GameModeRef`)))
    (:`then_1`
      (`self.HighlightHorizontalSquares` _color))
    (:`then_2`
      (`self.HighlightVerticalSquares` _color))
    (:`then_3`
      (return (`self.IsKing`)))))

(fn `UserConstructionScript`
  (`parent.UserConstructionScript`))